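; BP_EndStubuttons is an actor that judges the player's detention or signature decision on the student being diagnosed.
; It checks the disease manager's Faker flag, plus CureRight for signatures, then calls EventCured on the student and fires CORRECT or INCORRECT.
; Outcomes update local and game-instance tallies, and faker decisions shift the clamped BadStudents count.
; DayOneObjectGiven reuses the signature logic.
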(event `self.ReceiveBeginPlay`
  (bind _outactors (`GameplayStatics.GetAllActorsOfClass` "/Game/Blueprint/Actors/BP_Student.BP_Student_C"))
  (bind _outactors_2 (`GameplayStatics.GetAllActorsOfClass` "/Game/Blueprint/Actors/BP_DiseaseManager.BP_DiseaseManager_C"))
  (bind _returnvalue (`GameplayStatics.GetActorOfClass` "/Game/Blueprint/Actors/BP_CureObjects.BP_CureObjects_C"))
  (set `self.StuRef` (`|GetArrayItem` _outactors))
  (set `self.DiseaseManRef` (`|GetArrayItem` _outactors_2))
  (set `self.ObjectRef` _returnvalue)
  (set `self.CureRight` false)
  (bind _asbp_game_instance (cast `/Game/Blueprint/BP_GameInstance` (`GameplayStatics.GetGameInstance`)))
  (set `self.As BP Game Instance` _asbp_game_instance)
  (set `self.CorrectDetentions` 0)
  (set `self.CorrectCures` 0)
  (set `self.IncorrectCures` 0)
  (set `self.IncorrectDetentions` 0)
  (`KismetSystemLibrary.PrintString` (`KismetStringLibrary.Conv_IntToString` (`/Game/Blueprint/BP_GameInstance.Correct Cure` (`self.As BP Game Instance`)))))

(event `DetentionEvent`
  (bind _as_bp_game_instance (`self.As BP Game Instance`))
  (bind _sturef (`self.StuRef`))
  (if (`/Game/Blueprint/Actors/BP_Student.StudentDiagnosing` (`self.StuRef`))
    (if (`/Game/Blueprint/Actors/BP_DiseaseManager.Faker` (`self.DiseaseManRef`))
      (bind _output_get (set `/Game/Blueprint/Actors/BP_DiseaseManager.Bad students` (`KismetMathLibrary.Clamp` (- (stale _output_get) 1) 1 4) (`self.DiseaseManRef`)))
      (`/Game/Blueprint/Actors/BP_Student.EventCured` _sturef)
      (`KismetSystemLibrary.PrintString` "detention" true true (struct :`R` 1.0 :`G` 0.041028 :`A` 1.0))
      (`/Engine/EditorBlueprintResources/StandardMacros.IncrementInt` (`/Game/Blueprint/BP_GameInstance.Correct Detentions` _as_bp_game_instance)
        (:`  `
          (bind _output_get_2 (set `self.CorrectDetentions` (+ (stale _output_get_2) 1)))
          (`self.CORRECT`)))
      (else
        (`/Game/Blueprint/Actors/BP_Student.EventCured` _sturef)
        (`KismetSystemLibrary.PrintString` "actually sick" true true (struct :`R` 1.0 :`G` 0.49595 :`A` 1.0))
        (`/Engine/EditorBlueprintResources/StandardMacros.IncrementInt` (`/Game/Blueprint/BP_GameInstance.Needed Cure` _as_bp_game_instance)
          (:`  `
            (bind _output_get_3 (set `self.IncorrectDetentions` (+ (stale _output_get_3) 1)))
            (`self.INCORRECT`)))))))

(event `SignatureEvent`
  (bind _as_bp_game_instance (`self.As BP Game Instance`))
  (bind _diseasemanref (`self.DiseaseManRef`))
  (bind _sturef (`self.StuRef`))
  (if (`/Game/Blueprint/Actors/BP_Student.StudentDiagnosing` (`self.StuRef`)) :!label _label
    (if (not (`/Game/Blueprint/Actors/BP_DiseaseManager.Faker` _diseasemanref))
      (if (`self.CureRight`)
        (`/Game/Blueprint/Actors/BP_Student.EventCured` _sturef)
        (`KismetSystemLibrary.PrintString` "signature" true true (struct :`R` 0.015386 :`G` 1.0 :`A` 1.0))
        (`/Engine/EditorBlueprintResources/StandardMacros.IncrementInt` (`/Game/Blueprint/BP_GameInstance.Correct Cure` _as_bp_game_instance)
          (:`  `
            (bind _output_get (set `self.CorrectCures` (+ (stale _output_get) 1)))
            (`self.CORRECT`)))
        (else
          (`/Game/Blueprint/Actors/BP_Student.EventCured` _sturef)
          (`KismetSystemLibrary.PrintString` "wrong cure" true true (struct :`R` 1.0 :`G` 0.508791 :`A` 1.0))
          (`/Engine/EditorBlueprintResources/StandardMacros.IncrementInt` (`/Game/Blueprint/BP_GameInstance.Incorrect Cure` _as_bp_game_instance)
            (:`  `
              (bind _output_get_2 (set `self.IncorrectCures` (+ (stale _output_get_2) 1)))
              (`self.INCORRECT`)))))
      (else
        (bind _output_get_3 (set `/Game/Blueprint/Actors/BP_DiseaseManager.Bad students` (`KismetMathLibrary.Clamp` (+ (stale _output_get_3) 1) 1 4) _diseasemanref))
        (`/Game/Blueprint/Actors/BP_Student.EventCured` _sturef)
        (`KismetSystemLibrary.PrintString` "needed detention" true true (struct :`R` 1.0 :`G` 0.46368 :`A` 1.0))
        (`/Engine/EditorBlueprintResources/StandardMacros.IncrementInt` (`/Game/Blueprint/BP_GameInstance.Needed Detention` _as_bp_game_instance)
          (:`  `
            (bind _output_get_4 (set `self.IncorrectDetentions` (+ (stale _output_get_4) 1)))
            (`self.INCORRECT`)))))))

(event `DayOneObjectGiven`
  (goto _label))

(fn `UserConstructionScript`)