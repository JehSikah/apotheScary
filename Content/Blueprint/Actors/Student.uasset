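; Student actor, apparently an early test Blueprint for swapping a student's sprite through debug keys.
; Both keys overwrite the first StudentType struct entry with a "Doggy" label, a sprite and a flipbook.
; The first key also applies that sprite to the PaperSprite, sets its relative X from Speed, then decrements Speed.
; The second stores a dummy sprite without applying it; BeginPlay, Tick, overlap and construction are empty.
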(event EventBeginPlay)

(event Collision|EventActorBeginOverlap
  (params (OtherActor :type Actor%20Object%20Reference)))

(event EventTick
  (params (DeltaSeconds :type Float%20%28single-precision%29)))

(event Input|KeyboardEvents|DebugKey1
  (params (Key :type Key%20Structure :default "None") (ActionValue :type Input%20Action%20Value%20Structure))
  (bind _studenttype (Variables|Default|GetStudentType))
  (bind _output (Utilities|Array|Get(acopy) _studenttype))
  (:Pressed
    (|SetBy-RefVar _output (Utilities|Struct|MakeStudentTypeStruct "Doggy" "/Game/VisualAssets/Sprites/StudentSprites/Werewoof/WWTes_Sprite.WWTes_Sprite" "/Paper2D/Tutorial/Paper2D/TutorialAssets/TutorialFlipBook.TutorialFlipBook")) ; ???
    (bind _structout (Utilities|Struct|SetmembersinStudentTypeStruct _output)) ; One of these does something
    (Rendering|Components|Sprite|SetSprite (Variables|Default|GetPaperSprite) (.studentsprite _structout))
    (Transformation|SetRelativeLocation (Variables|Default|GetPaperSprite) (Math|Vector|MakeVector (Variables|Default|GetSpeed) 0.0 0.0) false false)
    (Variables|Default|SetSpeed (- (Variables|Default|GetSpeed) 1e+01))))

(event Input|KeyboardEvents|DebugKey2
  (params (Key :type Key%20Structure :default "None") (ActionValue :type Input%20Action%20Value%20Structure))
  (bind _studenttype (Variables|Default|GetStudentType))
  (bind _output (Utilities|Array|Get(acopy) _studenttype))
  (:Pressed
    (|SetBy-RefVar _output (Utilities|Struct|MakeStudentTypeStruct "Doggy" "/Paper2D/DummySprite.DummySprite" "/Paper2D/Tutorial/Paper2D/TutorialAssets/TutorialFlipBook.TutorialFlipBook")) ; ???
    (Utilities|Struct|SetmembersinStudentTypeStruct _output) ; One of these does something
  ))

(fn ConstructionScript)