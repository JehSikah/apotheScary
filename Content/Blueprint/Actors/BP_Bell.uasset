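; BP_Bell is a clickable paper-sprite bell that starts the game's BP_Timer when rung.
; Clicks are ignored during a BP_Principal penalty or tutorial, or while BP_Student is diagnosing; otherwise it plays a ding and fires its BellClicked dispatcher.
; Its own handler for that dispatcher starts the timer through a DoOnce, which the timer's completion event resets.
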(event `self.ReceiveBeginPlay`
  (bind _returnvalue (`GameplayStatics.GetActorOfClass` "/Game/Blueprint/Actors/BP_Student.BP_Student_C"))
  (bind _returnvalue_2 (`GameplayStatics.GetActorOfClass` "/Game/Blueprint/Actors/BP_Principal.BP_Principal_C"))
  (bind _returnvalue_3 (`GameplayStatics.GetActorOfClass` "/Game/Blueprint/Actors/BP_Timer.BP_Timer_C"))
  (add `/Game/Blueprint/Actors/BP_Timer.TimerCompleted` _returnvalue_3 (delegate `reset`))
  (add `self.BellClicked` (delegate `TImeStart`)))

(event `reset`
  (goto _label :!via `Reset`))

(event `TImeStart`
  (`/Engine/EditorBlueprintResources/StandardMacros.DoOnce` false :!label _label
    (:`Completed`
      (bind _returnvalue (`GameplayStatics.GetActorOfClass` "/Game/Blueprint/Actors/BP_Timer.BP_Timer_C"))
      (`/Game/Blueprint/Actors/BP_Timer.Timer Start` _returnvalue))))

(event `self.PaperSprite.OnClicked`
  (params (TouchedComponent :type "PrimitiveComponent Object Reference") (ButtonPressed :type "Key Structure"))
  (if (or (`/Game/Blueprint/Actors/BP_Principal.Penalty` (stale `self.ReceiveBeginPlay` _returnvalue_2)) (`/Game/Blueprint/Actors/BP_Principal.TutorialActive` (stale `self.ReceiveBeginPlay` _returnvalue_2)))
    _
    (elif (not (`/Game/Blueprint/Actors/BP_Student.StudentDiagnosing` (stale `self.ReceiveBeginPlay` _returnvalue)))
      (`GameplayStatics.PlaySound2D` "/Game/Sounds/ding.ding" 1.0 1.0 0.0 null null)
      (`self.BellClicked`))))

(fn `UserConstructionScript`)