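; Bp_Speech is an actor that displays a student's dialogue on a TextRender component in the world.
; On BeginPlay it hides the text and binds to the spawn-finish and cured dispatchers of the first BP_Student found.
; When spawning finishes, it copies CastedText from the first StudentDialogueWidget found and shows it.
; When the student is cured, it hides the text again.
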(event `ResetText`
  (`SceneComponent.SetHiddenInGame` (`self.TextRender`) true false))

(event `self.ReceiveBeginPlay`
  (bind _studentref (`self.StudentRef`))
  (`SceneComponent.SetHiddenInGame` (`self.TextRender`) true false)
  (bind _outactors (`GameplayStatics.GetAllActorsOfClass` "/Game/Blueprint/Actors/BP_Student.BP_Student_C"))
  (set `self.StudentRef` (`|GetArrayItem` _outactors))
  (add `/Game/Blueprint/Actors/BP_Student.SpawnFinishDispatch` _studentref (delegate `NewText`))
  (add `/Game/Blueprint/Actors/BP_Student.StudentCured` _studentref (delegate `ResetText`)))

(event `NewText`
  (bind _foundwidgets (`WidgetBlueprintLibrary.GetAllWidgetsOfClass` "/Game/Blueprint/Actors/StudentDialogueWidget.StudentDialogueWidget_C"))
  (bind _output_get (set `self.StudentDialogueRef` (`|GetArrayItem` _foundwidgets)))
  (`TextRenderComponent.K2_SetText` (`self.TextRender`) (`/Game/Blueprint/Actors/StudentDialogueWidget.CastedText` _output_get))
  (`SceneComponent.SetHiddenInGame` (`self.TextRender`) false false))

(fn `UserConstructionScript`)