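; School principal actor for a nurse game that appears at game or level start for the tutorial and pops up to penalize wrong answers.
; Binds to BP_Levels and BP_EndStubuttons events, reading the level number from BP_GameInstance.
; MoveComponentTo slides and flipbooks drive the entrance, penalty animation and randomized exit, with tutorial/penalty flags and start/over events signalling state.
; Tutorial dialogue lines remain as unconnected nodes.
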(event `self.ReceiveBeginPlay`
  (bind _returnvalue (`GameplayStatics.GetActorOfClass` "/Game/Blueprint/Actors/BP_Levels.BP_Levels_C"))
  (bind _output_get (set `self.LevelsRef` _returnvalue))
  (add `/Game/Blueprint/Actors/BP_Levels.GameStart` _output_get (delegate `NewGamePressed`))
  (add `/Game/Blueprint/Actors/BP_Levels.NewLevel` _output_get (delegate `NewLevel`))
  (bind _asbp_game_instance (cast `/Game/Blueprint/BP_GameInstance` (`GameplayStatics.GetGameInstance`)))
  (bind _output_get_2 (set `self.As BP Game Instance` _asbp_game_instance))
  (bind _output_get_3 (set `self.TutLevelNum` (`/Game/Blueprint/BP_GameInstance.LevelNum` _output_get_2)))
  (if (!= _output_get_3 0)
    (`self.NewLevel`)
    (`KismetSystemLibrary.PrintString` (`KismetStringLibrary.Conv_IntToString` _output_get_3) true true (struct :`R` 1.0 :`B` 0.102341 :`A` 1.0))
    (bind _outactors (`GameplayStatics.GetAllActorsOfClass` "/Game/Blueprint/Actors/BP_EndStubuttons.BP_EndStubuttons_C"))
    (add `/Game/Blueprint/Actors/BP_EndStubuttons.INCORRECT` _outactors (delegate `You did bad`))))

(event `NewGamePressed`
  (bind _thebigman (`self.TheBigMan`))
  (set `self.TutorialActive` true :!label _label)
  (`KismetSystemLibrary.Delay` 1.0)
  (`SceneComponent.SetVisibility` _thebigman true false)
  (set `self.TutLevelNum` (`/Game/Blueprint/BP_GameInstance.LevelNum` (stale `self.ReceiveBeginPlay` _asbp_game_instance)))
  (`PaperFlipbookComponent.SetFlipbook` (`self.theMan'sFB`) "/Game/VisualAssets/StuImgSeqs/_principalBigMan/principaldle.principaldle")
  (`KismetSystemLibrary.MoveComponentTo` _thebigman (400.0 -250.0 90.0) (struct :`Yaw` -90.0) true false 1.0)
  (`self.PrincipalEvent`))

(event `NewLevel`
  (goto _label))

(event `You did bad`
  (bind _thebigman (`self.TheBigMan`))
  (bind _theman_sfb (`self.theMan'sFB`))
  (set `self.Penalty` true)
  (`SceneComponent.SetWorldScale3D` (`self.theMan'sFB`) (`self.NewVar_0`))
  (`KismetSystemLibrary.MoveComponentTo` _thebigman (110.0 -250.0 63.0) (struct :`Yaw` 90.0) true false 0.0)
  (`PaperFlipbookComponent.SetFlipbook` _theman_sfb "/Game/VisualAssets/StuImgSeqs/_principalBigMan/WRONG/WRONGTEXT/WRONGCOLOR.WRONGCOLOR")
  (`PaperFlipbookComponent.PlayFromStart` _theman_sfb)
  (`SceneComponent.SetVisibility` _theman_sfb true false)
  (`KismetSystemLibrary.Delay` (`PaperFlipbookComponent.GetFlipbookLength` _theman_sfb))
  (`SceneComponent.SetVisibility` _theman_sfb true false)
  (`KismetSystemLibrary.MoveComponentTo` _thebigman (400.0 -800.0 90.0) (struct) false true 0.0)
  (set `self.Penalty` false))

(event `PrincipalLeave`
  (bind _thebigman (`self.TheBigMan`))
  (`/Engine/EditorBlueprintResources/StandardMacros.DoOnce` false
    (:`Completed`
      (bind _output_get (set `self.Rando` (`KismetMathLibrary.RandomInteger` 17)))
      (if (< _output_get 15)
        (`KismetSystemLibrary.MoveComponentTo` _thebigman (400.0 -800.0 90.0) (struct :`Yaw` -90.0) false true 1.0)
        (else
          (`KismetSystemLibrary.MoveComponentTo` _thebigman (400.0 -250.0 -250.0) (struct :`Yaw` -90.0) false true 2.5)))
      (`SceneComponent.SetVisibility` _thebigman false false)
      (set `self.TutorialActive` false)
      (`self.PrincipalOverEvent`))))

(fn `UserConstructionScript`)