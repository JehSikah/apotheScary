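; BP_Levels is an actor that handles level progression by reloading MainLevel for each new level.
; On BeginPlay it gets the game instance, finds the BP_Timer actor and binds to the NewLevel event.
; When that event fires, it increments the game instance's LevelNum unless at the cap, sets the timer's timespan and reopens the map.
; A debug key only prints text, and the save-game loading nodes are disconnected.
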(event Custom|NewLevel_Event
  (if (not (== (Variables|/Game/Blueprint/BP_GameInstance.BP_GameInstance_C|GetLevelNum (stale EventBeginPlay _asbp_game_instance)) 5))
    (Math|Integer|IncrementInt (Variables|/Game/Blueprint/BP_GameInstance.BP_GameInstance_C|GetLevelNum (stale EventBeginPlay _asbp_game_instance))
      (:%20%20
        (Variables|/Game/Blueprint/Actors/BP_Timer.BP_Timer_C|Settimespan (stale EventBeginPlay _output_get) (Math|Timespan|MakeTimespan 0 0 6))
        (Game|OpenLevel(byName) "MainLevel")))))

(event EventBeginPlay
  (bind _asbp_game_instance (Utilities|Casting|CastToBP_GameInstance (Game|GetGameInstance)))
  (bind _returnvalue (Actor|GetActorOfClass "/Game/Blueprint/Actors/BP_Timer.BP_Timer_C"))
  (bind _output_get (Variables|Default|SetTimerRef _returnvalue))
  (EventDispatchers|BindEventtoNewLevel (delegate Custom|NewLevel_Event)))

(event Input|KeyboardEvents|DebugKeyQ
  (params (Key :type Key%20Structure :default "None") (ActionValue :type Input%20Action%20Value%20Structure))
  (:Pressed
    (Development|PrintString (Utilities|String|ToString(Integer) 0) true true "(R=0.000000,G=1.000000,B=0.625059,A=1.000000)")))

(fn ConstructionScript)