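; BP_Book is a clickable book actor that opens the player's book interface.
; Clicking its Sphere component sets BookOpen, then hides HistoryUI and shows BookUI on the BP_PlayerChar.
; It also spawns a THE_WALL actor at a fixed world-X offset from the camera location, regardless of where the camera faces.
; The file contains no logic for closing the book or removing the wall.
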(event `self.Sphere.OnClicked`
  (params (TouchedComponent :type "PrimitiveComponent Object Reference") (ButtonPressed :type "Key Structure"))
  (set `self.BookOpen` true)
  (bind _asbp_player_char (cast `/Game/Blueprint/Actors/BP_PlayerChar` (`GameplayStatics.GetPlayerCharacter` 0)))
  (`Widget.SetVisibility` (`/Game/Blueprint/Actors/BP_PlayerChar.History UI` _asbp_player_char) "Hidden")
  (`Widget.SetVisibility` (`/Game/Blueprint/Actors/BP_PlayerChar.BookUI` _asbp_player_char) "Visible")
  (`|SpawnActorFromClass` "/Game/Blueprint/Actors/THE_WALL.THE_WALL_C" (`KismetMathLibrary.MakeTransform` (+ (`PlayerCameraManager.GetCameraLocation` (`GameplayStatics.GetPlayerCameraManager` 0)) (100.0 0.0 0.0))) "Undefined" "MultiplyWithRoot" null null))

(fn `UserConstructionScript`)