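; BP_Student is the 2D student patient that appears, gets diagnosed and is cured.
; BeginPlay caches BP_DiseaseManager and loads student and disease DataTable rows into arrays.
; SpawnStudent picks a random student look, copies disease and cure from the manager unless it flags a faker, moves the sprite in and creates a hidden dialogue widget.
; EventCured slides the student away and respawns another; debug keys trigger cures and printouts.
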(event Custom|ResetStudent
  ;[0.15 0.15 0.15 0.5] Reset the Student
  (Rendering|SetVisibility (Variables|Default|GetPaperSprite) false false)
  (Components|MoveComponentTo (Variables|Default|GetPaperSprite) "400.000000,300.000000,0.000000" "0.000000,90.000000,0.000000" true false 0.0 false)
  (Variables|Default|SetStudentDiagnosing false)
  (Utilities|FlowControl|Delay 0.0)
  (CallFunction|SpawnStudent))

(event Custom|EventCured
  ;[0.15 0.15 0.15 0.5] Cure Student Event
  (Default|CallStudentCured)
  (if (not (Variables|Default|GetStudentMoveActive))
    (if (Variables|Default|GetStudentDiagnosing)
      (Widget|RemovefromParent (Variables|Default|GetDialogue%20Widget))
      (Components|MoveComponentTo (Variables|Default|GetPaperSprite) "400.000000,-800.000000,0.000000" "0.000000,90.000000,0.000000" true false 2.0 false)
      (Utilities|FlowControl|Delay 2.0)
      (CallFunction|ResetStudent))))

(event Custom|SpawnStudent
  ;[0.15 0.15 0.15 0.5] Spawn Student
  (if (not (Variables|Default|GetStudentMoveActive))
    (if (not (Variables|Default|GetStudentDiagnosing))
      (Variables|Default|SetStudentDiagnosing true)
      (Variables|Default|SetStudentRowPick (Math|Random|RandomInteger 5))
      (Variables|Default|SetStudentRefEnum (.StudentTypeString (Utilities|Struct|BreakSTR_StudentInfo (Utilities|Array|Get(acopy) (Variables|Default|GetStudentType) (Variables|Default|GetStudentRowPick)))))
      (Default|CallStudentSpawning)
      (Variables|Default|SetStudentTypeString (Utilities|String|EnumtoString (.StudentTypeString (Utilities|Struct|BreakSTR_StudentInfo (Utilities|Array|Get(acopy) (Variables|Default|GetStudentType) (Variables|Default|GetStudentRowPick))))))
      (Rendering|SetVisibility (Variables|Default|GetPaperSprite) true false)
      (Sprite|SetFlipbook (Variables|Default|GetPaperFlipbook) (.StudentFlipbook (Utilities|Struct|BreakSTR_StudentInfo (Utilities|Array|Get(acopy) (Variables|Default|GetStudentType) (Variables|Default|GetStudentRowPick)))))
      (Rendering|Components|Sprite|SetSprite (Variables|Default|GetPaperSprite) (.StudentSprite (Utilities|Struct|BreakSTR_StudentInfo (Utilities|Array|Get(acopy) (Variables|Default|GetStudentType) (Variables|Default|GetStudentRowPick)))))
      (bind _asbp_disease_manager (Utilities|Casting|CastToBP_DiseaseManager (Variables|Default|GetDiseasemanagerref)))
      (if (Variables|/Game/Blueprint/Actors/BP_DiseaseManager.BP_DiseaseManager_C|GetFaker _asbp_disease_manager)
        (Development|PrintString "yahoooyippeeehorrayyyy\\")
        (Variables|Default|SetStudentMoveActive true)
        (Components|MoveComponentTo (Variables|Default|GetPaperSprite) "400.000000,-250.000000,0.000000" "0.000000,90.000000,0.000000" true false 0.0 false)
        (Variables|Default|SetStudentMoveActive false)
        (CallFunction|SpawnFinished)
        (Default|CallSpawnFinishDispatch)
        (else
          (bind _asbp_disease_manager_2 (Utilities|Casting|CastToBP_DiseaseManager (Variables|Default|GetDiseasemanagerref))
            (:then
              (Variables|Default|SetDisease (Variables|/Game/Blueprint/Actors/BP_DiseaseManager.BP_DiseaseManager_C|GetManagerDisease _asbp_disease_manager_2))
              (Variables|Default|SetCurrent%20Cure (Variables|/Game/Blueprint/Actors/BP_DiseaseManager.BP_DiseaseManager_C|GetManagherCure _asbp_disease_manager_2))
              (Variables|Default|SetCureEnumRef (Variables|/Game/Blueprint/Actors/BP_DiseaseManager.BP_DiseaseManager_C|GetCureEnumRef _asbp_disease_manager_2))
              (Variables|Default|SetStudentMoveActive true)
              (Components|MoveComponentTo (Variables|Default|GetPaperSprite) "400.000000,-250.000000,0.000000" "0.000000,90.000000,0.000000" true false 0.0 false)
              (Variables|Default|SetStudentMoveActive false)
              (CallFunction|SpawnFinished)
              (Development|PrintString (Utilities|String|EnumtoString (.StudentTypeString (Utilities|Struct|BreakSTR_StudentInfo (Utilities|Array|Get(acopy) (Variables|Default|GetStudentType) (Variables|Default|GetStudentRowPick))))))
              (Default|CallSpawnFinishDispatch))
            (:CastFailed
              (Development|PrintString "fuck fuck fuck fuck"))))))))

(event Custom|SpawnFinished
  (Development|PrintString "Tried my best")
  (bind _returnvalue (UserInterface|CreateWidget "/Game/Blueprint/Actors/StudentDialogueWidget.StudentDialogueWidget_C"))
  (bind _output_get (Variables|Default|SetDialogue%20Widget _returnvalue))
  (UserInterface|Viewport|AddtoViewport _output_get 0)
  (Widget|SetVisibility _output_get "Hidden"))

(event EventBeginPlay
  (bind _diseaseref (Variables|Default|GetDiseaseRef))
  (bind _studentinforef (Variables|Default|GetStudentInfoRef))
  ;[0.15 0.15 0.15 0.5] Sets struct data by DataTable date her.
  (bind _outactors (Actor|GetAllActorsOfClass "/Game/Blueprint/Actors/BP_DiseaseManager.BP_DiseaseManager_C"))
  (Variables|Default|SetDiseasemanagerref (Utilities|Array|Get(acopy) _outactors))
  (bind _outrownames (DataTable|GetDataTableRowNames _studentinforef))
  (for _array_element _outrownames
    (bind _returnvalue (Utilities|GetDataTableRow _studentinforef _array_element)
      (:then
        (Utilities|Array|Add (Variables|Default|GetStudentType) _returnvalue)
        (bind _outrownames_2 (DataTable|GetDataTableRowNames _diseaseref))
        (for _array_element_2 _outrownames_2
          (bind _returnvalue_2 (Utilities|GetDataTableRow _diseaseref _array_element_2)
            (:then
              (Utilities|Array|Add (Variables|Default|GetDiseaseType) _returnvalue_2))))))))

(event Collision|EventActorBeginOverlap
  (params (OtherActor :type Actor%20Object%20Reference)))

(event Input|KeyboardEvents|DebugKey1
  (params (Key :type Key%20Structure :default "None") (ActionValue :type Input%20Action%20Value%20Structure))
  ;[0.15 0.15 0.15 0.5] Spawn Student
)

(event Input|KeyboardEvents|DebugKeyM
  (params (Key :type Key%20Structure :default "None") (ActionValue :type Input%20Action%20Value%20Structure))
  (:Pressed
    (Utilities|FlowControl|FlipFlop
      (:A
        (Variables|Default|SetTextTalk false)
        (Development|PrintString "TALK"))
      (:B
        (Variables|Default|SetTextTalk true)
        (Development|PrintString "NOTALK")))))

(event Input|KeyboardEvents|DebugKey4
  (params (Key :type Key%20Structure :default "None") (ActionValue :type Input%20Action%20Value%20Structure))
  (:Pressed
    (Development|PrintString (Variables|Default|GetDisease)))
  (:Released
    (Development|PrintString (Variables|Default|GetCurrent%20Cure))))

(event Input|KeyboardEvents|DebugKey2
  (params (Key :type Key%20Structure :default "None") (ActionValue :type Input%20Action%20Value%20Structure))
  ;[0.15 0.15 0.15 0.5] Cure Student Event
  (:Pressed
    (CallFunction|EventCured)))

(fn ConstructionScript)

(fn Hunterscoolfunction
  (params (Object :type Object%20Object%20Reference))
  (Development|PrintString "FUUUCK YEAAAAHH BABBYYYYYY"))