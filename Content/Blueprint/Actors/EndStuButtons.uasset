(event `self.ReceiveBeginPlay`
  (bind _outactors (`GameplayStatics.GetAllActorsOfClass` "/Game/Blueprint/Actors/BP_Student.BP_Student_C"))
  (bind _outactors_2 (`GameplayStatics.GetAllActorsOfClass` "/Game/Blueprint/Actors/BP_DiseaseManager.BP_DiseaseManager_C"))
  (bind _returnvalue (`GameplayStatics.GetActorOfClass` "/Game/Blueprint/Actors/Object_test.Object_test_C"))
  (set `self.StuRef` (`|GetArrayItem` _outactors))
  (set `self.DiseaseManRef` (`|GetArrayItem` _outactors_2))
  (set `self.ObjectRef` _returnvalue)
  (set `self.CureRight` false))

(event `DetentionEvent`
  (bind _sturef (`self.StuRef`))
  (if (`/Game/Blueprint/Actors/BP_DiseaseManager.Faker` (`self.DiseaseManRef`))
    (bind _output_get (set `/Game/Blueprint/Actors/BP_DiseaseManager.Bad students` (`KismetMathLibrary.Clamp` (- (stale _output_get) 1) 1 4) (`self.DiseaseManRef`)))
    (`/Game/Blueprint/Actors/BP_Student.EventCured` _sturef)
    (`KismetSystemLibrary.PrintString` "detention" true true (struct :`R` 1.0 :`G` 0.041028 :`A` 1.0))
    (else
      (`/Game/Blueprint/Actors/BP_Student.EventCured` _sturef)
      (`KismetSystemLibrary.PrintString` "actually sick" true true (struct :`R` 1.0 :`G` 0.49595 :`A` 1.0)))))

(event `self.Detention.OnClicked`
  (params (TouchedComponent :type "PrimitiveComponent Object Reference") (ButtonPressed :type "Key Structure")))

(event `self.detentioncube.OnClicked`
  (params (TouchedComponent :type "PrimitiveComponent Object Reference") (ButtonPressed :type "Key Structure")))

(event `self.Signature.OnClicked`
  (params (TouchedComponent :type "PrimitiveComponent Object Reference") (ButtonPressed :type "Key Structure")))

(event `SignatureEvent`
  (bind _sturef (`self.StuRef`))
  (bind _diseasemanref (`self.DiseaseManRef`))
  (if (not (`/Game/Blueprint/Actors/BP_DiseaseManager.Faker` _diseasemanref))
    (if (`self.CureRight`)
      (`/Game/Blueprint/Actors/BP_Student.EventCured` _sturef)
      (`KismetSystemLibrary.PrintString` "signature" true true (struct :`R` 0.015386 :`G` 1.0 :`A` 1.0))
      (else
        (`/Game/Blueprint/Actors/BP_Student.EventCured` _sturef)
        (`KismetSystemLibrary.PrintString` "wrong cure" true true (struct :`R` 1.0 :`G` 0.508791 :`A` 1.0))))
    (else
      (bind _output_get (set `/Game/Blueprint/Actors/BP_DiseaseManager.Bad students` (`KismetMathLibrary.Clamp` (+ (stale _output_get) 1) 1 4) _diseasemanref))
      (`/Game/Blueprint/Actors/BP_Student.EventCured` _sturef)
      (`KismetSystemLibrary.PrintString` "needed detention" true true (struct :`R` 1.0 :`G` 0.46368 :`A` 1.0)))))

(event `self.signaturecube.OnClicked`
  (params (TouchedComponent :type "PrimitiveComponent Object Reference") (ButtonPressed :type "Key Structure")))

(fn `UserConstructionScript`)