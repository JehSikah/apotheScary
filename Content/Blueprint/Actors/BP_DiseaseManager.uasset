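; Disease manager actor that assigns each spawned student either a real disease with cure and symptoms, or a faked illness cured by Detention.
; On BeginPlay it caches steward, faker and disease DataTable rows in nested loops and binds to the student's spawn event.
; Fakers are rolled randomly, except on tutorial level 1.
; Real diseases are re-rolled through a self-bound dispatcher until compatible with the student type for that level; debugging starts from a fixed row.
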(event `self.ReceiveBeginPlay`
  (bind _diseasetableref (`self.DiseaseTableRef`))
  (bind _faker_table_ref (`self.Faker Table Ref`))
  (bind _stewards_reference (`self.Stewards Reference`))
  (add `self.GetValidDispatch` (delegate `GetValidDisease`))
  (bind _outactors (`GameplayStatics.GetAllActorsOfClass` "/Game/Blueprint/Actors/BP_Student.BP_Student_C"))
  (set `self.StuRef` (`|GetArrayItem` _outactors))
  (bind _returnvalue (`GameplayStatics.GetActorOfClass` "/Game/Blueprint/Actors/BP_Principal.BP_Principal_C"))
  (set `self.TutorialRef` _returnvalue)
  (bind _outrownames (`DataTableFunctionLibrary.GetDataTableRowNames` _stewards_reference))
  (for _array_element _outrownames
    (bind _returnvalue_2 (`|GetDataTableRow` _stewards_reference _array_element)
      (:`then`
        (`KismetArrayLibrary.Array_Add` (`self.StuSTRRef`) _returnvalue_2)
        (bind _outrownames_2 (`DataTableFunctionLibrary.GetDataTableRowNames` _faker_table_ref))
        (for _array_element_2 _outrownames_2
          (bind _returnvalue_3 (`|GetDataTableRow` _faker_table_ref _array_element_2)
            (:`then`
              (`KismetArrayLibrary.Array_Add` (`self.Faker STR Ref`) _returnvalue_3)
              (bind _outrownames_3 (`DataTableFunctionLibrary.GetDataTableRowNames` _diseasetableref))
              (for _array_element_3 _outrownames_3
                (bind _returnvalue_4 (`|GetDataTableRow` _diseasetableref _array_element_3)
                  (:`then`
                    (`KismetArrayLibrary.Array_Add` (`self.DiseaseStrRef`) _returnvalue_4)
                    (if (== (`/Game/Blueprint/Actors/BP_Principal.TutLevelNum` (`self.TutorialRef`)) 1)
                      (set `self.Bad students` -1)
                      (else
                        (set `self.Bad students` 1)))
                    (add `/Game/Blueprint/Actors/BP_Student.StudentSpawning` (`self.StuRef`) (delegate `StudentSpawned`))))))))))))

(event `StudentSpawned`
  (bind _sturef (`self.StuRef`))
  (bind (_diseaseenum _diseasename _symptom1 _symptom2 _symptom3 _cure) (break `/Game/Blueprint/Data-Structs/STR_Disease` (`|GetArrayItem` (`self.DiseaseStrRef`) (`self.DiseaseRowPick`))))
  (if (<= (`KismetMathLibrary.RandomInteger` 10) (`self.Bad students`))
    (set `self.Faker` true)
    (`KismetSystemLibrary.PrintString` "Faker")
    (set `self.Faker Row Pick` (`KismetMathLibrary.RandomInteger` 3))
    (set `self.FakerDisease` "Fake")
    (set `self.ManagerDisease` "Faker")
    (set `self.ManagherCure` "Detention")
    (else
      (set `self.Faker` false)
      (if (`/Game/Blueprint/Actors/BP_Student.Debugging` (`self.StuRef`))
        (set `self.DiseaseRowPick` 3)
        (set `self.CureEnumRef` _cure :!label _label)
        (set `self.ManagherCure` (`|GetEnumeratorNameAsString` _cure))
        (set `self.ManagerDisease` _diseasename)
        (set `self.Disease Enum` _diseaseenum)
        (set `self.ManagherType` (`/Game/Blueprint/Actors/BP_Student.StudentTypeString` _sturef))
        (bind _output_get (set `self.SymptomArray` (`|MakeArray` _symptom1 _symptom2 _symptom3)))
        (if (`KismetStringLibrary.Contains` (`BlueprintMapLibrary.Map_Find` (`.StudentsCompatibility_10_27B50A40464E6AECF14FEF89931B07F4` (break `/Game/Blueprint/Data-Structs/STR_NestedStu` (`BlueprintMapLibrary.Map_Find` (`.Students_7_7194FB7D4E471602DD1084BF5FD6D793` (break `/Game/Blueprint/Data-Structs/STR_Stu` (`|GetArrayItem` (`self.StuSTRRef`)))) (`/Game/Blueprint/Actors/BP_Principal.TutLevelNum` (`self.TutorialRef`))))) (`/Game/Blueprint/Actors/BP_Student.StudentRefEnum` _sturef)) (`self.ManagerDisease`))
          (`KismetSystemLibrary.PrintString` "VALIDDISASE" true true (struct :`G` 1.0 :`B` 0.207035 :`A` 1.0) 8.0)
          (else
            (`KismetSystemLibrary.PrintString` "INVALIDISEASE" true true (struct :`R` 1.0 :`G` 0.456482 :`A` 1.0) 8.0)
            (`self.GetValidDispatch`)))
        (else
          (`self.GetValidDispatch`))))))

(event `GetValidDisease`
  (`KismetSystemLibrary.PrintString` "REAL")
  (set `self.DiseaseRowPick` (`KismetMathLibrary.RandomInteger` (`KismetArrayLibrary.Array_Length` (`self.DiseaseStrRef`))))
  (goto _label))

(fn `UserConstructionScript`)