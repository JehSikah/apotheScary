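; Dialogue manager that picks a student's intro line and outcome texts, depending on whether the student is faking or sick.
; On BeginPlay it caches the disease manager, questionnaire and student, loads misc table rows, and binds to the student's spawn-finish dispatcher.
; On spawn, student type keys the lookups: fakers get a random questionnaire intro, sick students one of three "$"-split symptom phrases.
; It then calls CallTextSet; key 7 debug-prints the intro.
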(event Custom|CustomEvent
  (bind _miscref (Variables|Default|GetMiscRef))
  (bind _student_refer (Variables|Default|GetStudent%20Refer))
  (bind _diseasemanagerref (Variables|Default|GetDiseaseManagerRef))
  (bind _questionref (Variables|Default|GetQuestionref))
  (bind _output (Utilities|Array|Get(acopy) _miscref))
  (bind _studenttype (Variables|/Game/Blueprint/Actors/BP_Student.BP_Student_C|GetStudentType _student_refer))
  (bind _diseasestrref (Variables|/Game/Blueprint/Actors/BP_DiseaseManager.BP_DiseaseManager_C|GetDiseaseStrRef _diseasemanagerref))
  (bind _studentrowpick (Variables|/Game/Blueprint/Actors/BP_Student.BP_Student_C|GetStudentRowPick _student_refer))
  (bind _diseaserowpick (Variables|/Game/Blueprint/Actors/BP_DiseaseManager.BP_DiseaseManager_C|GetDiseaseRowPick _diseasemanagerref))
  (bind _str_faleranswersref (Variables|/Game/Blueprint/Actors/BP_Questionaire.BP_Questionaire_C|GetSTR_FalerAnswersRef _questionref))
  (bind _numeratormap (Utilities|Struct|BreakSTR_MiscDialogue _output))
  (bind _output_2 (Utilities|Array|Get(acopy) _studenttype _studentrowpick))
  (bind _output_3 (Utilities|Array|Get(acopy) _diseasestrref _diseaserowpick))
  (bind _output_4 (Utilities|Array|Get(acopy) _str_faleranswersref))
  (bind _studenttypestring (Utilities|Struct|BreakSTR_StudentInfo _output_2))
  (bind _sympt1_syntax (Utilities|Struct|BreakSTR_Disease _output_3))
  (bind _numeratormap_2 (Utilities|Struct|BreakSTR_FakerAnswers _output_4))
  (bind _value (Utilities|Map|Find _sympt1_syntax _studenttypestring))
  (bind _value_2 (Utilities|Map|Find _numeratormap _studenttypestring))
  (bind _value_3 (Utilities|Map|Find _numeratormap_2 _studenttypestring))
  (bind _introdialogue (Utilities|Struct|BreakSTR_FakerStrings _value_3))
  (bind (_cured _sickdetention _detentionright _fakerwalksfree) (Utilities|Struct|BreakSTR_MiscStrings _value_2))
  (bind (_lefts _rights) (Utilities|String|Split _value "$"))
  (bind (_lefts_2 _rights_2) (Utilities|String|Split _rights "$"))
  (bind _array (Utilities|Array|MakeArray _lefts _lefts_2 _rights_2))
  (if (Variables|/Game/Blueprint/Actors/BP_DiseaseManager.BP_DiseaseManager_C|GetFaker _diseasemanagerref)
    (Variables|Default|SetFakerFree _fakerwalksfree)
    (Variables|Default|SetDetentionRight _detentionright)
    (bind _output_get (Variables|Default|SetStudentEntranceInt (Math|Random|RandomInteger (Utilities|Array|Length _introdialogue))))
    (Variables|Default|SetintroText (Utilities|Array|Get(acopy) _introdialogue _output_get))
    (Default|CallTextSet)
    (else
      (Variables|Default|SetSickDetention _sickdetention)
      (Variables|Default|SetCuredRight _cured)
      (Variables|Default|SetStudentEntranceInt (Math|Random|RandomInteger (Utilities|Array|Length _array)))
      (bind _output_get_2 (Variables|Default|SetintroText (Utilities|Array|Get(acopy) _array (Variables|Default|GetStudentEntranceInt))))
      (Default|CallTextSet))))

(event EventBeginPlay
  (bind _misctableref (Variables|Default|GetMiscTableRef))
  (bind _outactors (Actor|GetAllActorsOfClass "/Game/Blueprint/Actors/BP_DiseaseManager.BP_DiseaseManager_C"))
  (Variables|Default|SetDiseaseManagerRef (Utilities|Array|Get(acopy) _outactors))
  (Utilities|Casting|CastToBP_DiseaseManager (Variables|Default|GetDiseaseManagerRef))
  (bind _returnvalue (Actor|GetActorOfClass "/Game/Blueprint/Actors/BP_Questionaire.BP_Questionaire_C"))
  (Variables|Default|SetQuestionref _returnvalue)
  (bind _outactors_2 (Actor|GetAllActorsOfClass "/Game/Blueprint/Actors/BP_Student.BP_Student_C"))
  (bind _output_get (Variables|Default|SetStudent%20Refer (Utilities|Array|Get(acopy) _outactors_2)))
  (bind _outrownames (DataTable|GetDataTableRowNames _misctableref))
  (for _array_element _outrownames
    (bind _returnvalue_2 (Utilities|GetDataTableRow _misctableref _array_element)
      (:then
        (Utilities|Array|Add (Variables|Default|GetMiscRef) _returnvalue_2)
        (bind _asbp_student (Utilities|Casting|CastToBP_Student _output_get)
          (:then
            (EventDispatchers|BindEventtoSpawnFinishDispatch _asbp_student (delegate Custom|CustomEvent)))
          (:CastFailed
            (Development|PrintString "McFuck")))))))

(event Input|KeyboardEvents|DebugKey7
  (params (Key :type Key%20Structure :default "None") (ActionValue :type Input%20Action%20Value%20Structure))
  (:Pressed
    (Development|PrintString (stale Custom|CustomEvent _output_get_2))))

(fn ConstructionScript)