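; AC_ObjectPool is an object pool that pre-spawns actors of a configurable class for reuse.
; On BeginPlay it spawns a batch sized by PooledSize, stores them in ObjectPool and marks each as not in use.
; SpawnFromPool linearly searches for the first free actor, moves it to the requested transform and marks it in use.
; The pool never grows, printing a failure message when no free actor is found.
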(event `self.ReceiveBeginPlay`
  (`self.IntializePool`))

(event `IntializePool`
  (for _ (range (+ (`self.PooledSize`) 1))
    (bind _returnvalue (`|SpawnActorFromClass` (`self.PooledActorClass`) (`KismetMathLibrary.MakeTransform` (0.0 0.0 0.0)) "Undefined" "MultiplyWithRoot" null 0.0 null))
    (`KismetArrayLibrary.Array_AddUnique` (`self.ObjectPool`) _returnvalue)
    (`/Game/Blueprint/Actors/BP_PooledActor.SetInUse` _returnvalue false)))

(fn `FindFirstAvailibleActor`
  (returns (PooledActor :type "/Game/Blueprint/Actors/BP_PooledActor Object Reference"))
  (for _array_element (`self.ObjectPool`)
    (if (not (`/Game/Blueprint/Actors/BP_PooledActor.inUse` _array_element))
      (return null))))

(fn `SpawnFromPool`
  (params (SpawnTransform :type "Transform Structure"))
  (returns (PooledActor :type "/Game/Blueprint/Actors/BP_PooledActor Object Reference"))
  (bind _pooledactor (`self.FindFirstAvailibleActor`))
  (`/Engine/EditorBlueprintResources/StandardMacros.IsValid` _pooledactor
    (:`Is Valid`
      (`Actor.K2_SetActorTransform` _pooledactor SpawnTransform false false)
      (`/Game/Blueprint/Actors/BP_PooledActor.SetInUse` _pooledactor true)
      (return _pooledactor))
    (:`Is Not Valid`
      (`KismetSystemLibrary.PrintString` "Failed to spawn actor"))))