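; Draggable cure item that the player picks up and drops on a student to treat them.
; Loads its type from a data table, then compares it to the student's cure or fires water tutorial events on BP_Prinicipal.
; BP_Storage dispatchers reveal fridge and cupboard items, which are otherwise hidden and parked away.
; Tick handles mouse-following and right-click inspection before a spawned wall, where clicking flips the flipbook sprite via timelines.
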(event `self.Cube.OnClicked`
  (params (TouchedComponent :type "PrimitiveComponent Object Reference") (ButtonPressed :type "Key Structure"))
  (bind (_frideitems _cupboarditems) (`self.ItemsInStorage`))
  (bind _item_sprite (`self.Item_Sprite`))
  (bind _storageref (`self.StorageRef`))
  (bind (_curetype _flipbook _flipbookass) (break `/Game/Blueprint/Data-Structs/STR_Cures` (`|GetArrayItem` (`self.Cure Type`) (`self.CureNumber`))))
  ; I want that thing
  (if (`self.bIsDragging`)
    _
    (elif (`self.Inspecting`)
      ; Get Rotated Imbecile
      (if (`self.Flipped`)
        (set `self.Flipped` false)
        (bind (_direction _newtrack_0) (`Timeline|Get Rotated AGAIN Idiot` :!via `PlayFromStart`)
          (:`Update`
            (`SceneComponent.K2_SetRelativeRotation` _item_sprite (`KismetMathLibrary.RLerp` (struct :`Yaw` 90.0) (struct :`Yaw` 180.0) _newtrack_0) false false)
            (`KismetSystemLibrary.Delay` 0.2)
            (`PaperFlipbookComponent.SetFlipbook` _item_sprite _flipbook)
            (bind (_direction_2 _newtrack_0_2) (`Timeline|Timeline_1` :!via `PlayFromStart`)
              (:`Update`
                (`SceneComponent.K2_SetRelativeRotation` _item_sprite (`KismetMathLibrary.RLerp` (struct :`Yaw` 180.0) (struct :`Yaw` 90.0) _newtrack_0_2) false false)))))
        (else
          (set `self.Flipped` true)
          (bind (_direction_3 _newtrack_0_3) (`Timeline|Get Rotated Idiot` :!via `PlayFromStart`)
            (:`Update`
              (`SceneComponent.K2_SetRelativeRotation` _item_sprite (`KismetMathLibrary.RLerp` (struct :`Yaw` 90.0) (struct :`Yaw` 180.0) _newtrack_0_3) false false)
              (`KismetSystemLibrary.Delay` 0.2)
              (`PaperFlipbookComponent.SetFlipbook` _item_sprite _flipbookass)
              (bind (_direction_4 _newtrack_0_4) (`Timeline|Timeline` :!via `PlayFromStart`)
                (:`Update`
                  (`SceneComponent.K2_SetRelativeRotation` _item_sprite (`KismetMathLibrary.RLerp` (struct :`Yaw` 180.0) (struct :`Yaw` 90.0) _newtrack_0_4) false false)))))))
      (else
        (`|ExecutionSequence`
          (:`then_1`
            (set `self.bIsDragging` true)
            (set `self.AtOrigin` false)
            (bind (_direction_5 _newtrack_1) (`Timeline|Grab Tick` :!via `PlayFromStart`)
              (:`Update`
                (`SceneComponent.K2_SetRelativeRotation` (`self.Item_Sprite`) (`KismetMathLibrary.RLerp` (struct :`Yaw` 90.0) (struct :`Pitch` 20.0 :`Yaw` 90.0) _newtrack_1) false false))))
          (:`then_2`
            (if _frideitems
              (`/Game/Blueprint/Actors/BP_Storage.OpeningFridge` _storageref)
              (`|ExecutionSequence` :!label _label
                (:`then_0`
                  (`PaperFlipbookComponent.SetFlipbook` (`/Game/Blueprint/Actors/BP_Storage.Drawers` _storageref) "/Game/VisualAssets/WorldSprites/FB_CupboardClosed.FB_CupboardClosed")
                  (set `/Game/Blueprint/Actors/BP_Storage.CupboardOpen` false _storageref))
                (:`then_1`
                  (`PaperFlipbookComponent.SetFlipbook` (`/Game/Blueprint/Actors/BP_Storage.Fridge` _storageref) "/Game/VisualAssets/WorldSprites/FB_FridgeClosed.FB_FridgeClosed")
                  (set `/Game/Blueprint/Actors/BP_Storage.FridgeOpen` false _storageref)))
              (elif _cupboarditems
                (`/Game/Blueprint/Actors/BP_Storage.OpeningDrawer` _storageref)
                (goto _label))))
          (:`then_3`
            (`SceneComponent.SetVisibility` (`self.Item_Sprite`) true false)))))))

(event `self.ReceiveBeginPlay`
  (bind (_frideitems _cupboarditems) (`self.ItemsInStorage`))
  (bind _curetableref (`self.CureTableRef`))
  (bind (_curetype _flipbook _flipbookass) (break `/Game/Blueprint/Data-Structs/STR_Cures` (`|GetArrayItem` (`self.Cure Type`) (`self.CureNumber`))))
  ; find object starting point
  (bind _returnvalue (`GameplayStatics.GetActorOfClass` "/Game/Blueprint/Actors/BP_Prinicipal.BP_Prinicipal_C"))
  (set `self.TutRef` _returnvalue)
  (bind _returnvalue_2 (`GameplayStatics.GetActorOfClass` "/Game/Blueprint/Actors/BP_EndStubuttons.BP_EndStubuttons_C"))
  (set `self.EndStuButRef` _returnvalue_2)
  (bind _returnvalue_3 (`GameplayStatics.GetActorOfClass` "/Game/Blueprint/Actors/BP_Storage.BP_Storage_C"))
  (bind _output_get (set `self.StorageRef` _returnvalue_3))
  (add `/Game/Blueprint/Actors/BP_Storage.OpeningFridge` _output_get (delegate `UnhideFridgeItems`))
  (add `/Game/Blueprint/Actors/BP_Storage.OpeningDrawer` _output_get (delegate `UnhideDrawerItems`))
  (set `self.Object Origin` (`self.K2_GetActorLocation` (`ActorComponent.GetOwner` (`self.Cube`))))
  ; Set Cure Type
  (bind _outrownames (`DataTableFunctionLibrary.GetDataTableRowNames` _curetableref))
  (for _array_element _outrownames
    (bind _returnvalue_4 (`|GetDataTableRow` _curetableref _array_element)
      (:`then`
        (`KismetArrayLibrary.Array_Add` (`self.Cure Type`) _returnvalue_4))))
  (set `self.Cure` (`|GetEnumeratorNameAsString` _curetype))
  (`PaperFlipbookComponent.SetFlipbook` (`self.Item_Sprite`) _flipbook)
  (if (or _frideitems _cupboarditems)
    (`SceneComponent.SetVisibility` (`self.Item_Sprite`) false false)
    (`SceneComponent.K2_SetWorldLocation` (`self.Cube`) (0.0 1000.0 0.0) false false)))

(event `self.ReceiveActorBeginCursorOver`
  ; over or under
  (set `self.MouseOver` true)
  ; Make him Big
  (if (not (`self.Inspecting`))
    (`SceneComponent.SetRelativeScale3D` (`self.Cube`) (0.8 0.8 0.8))
    (`self.SetActorTickEnabled` true)))

(event `self.ReceiveActorEndCursorOver`
  ; over or under
  (set `self.MouseOver` false)
  ; Make him Big
  (if (not (`self.Inspecting`))
    (`SceneComponent.SetRelativeScale3D` (`self.Cube`) (0.5 0.5 0.5))))

(event `UnhideFridgeItems`
  (bind _item_sprite (`self.Item_Sprite`))
  (bind _object_origin (`self.Object Origin`))
  (bind _cube (`self.Cube`))
  (bind _returnvalue (and (not (`self.MouseOver`)) (`self.ItemsInStorage`)))
  (`/Engine/EditorBlueprintResources/StandardMacros.FlipFlop`
    (:`A`
      (if _returnvalue
        (`SceneComponent.K2_SetWorldLocation` _item_sprite _object_origin false false :!label _label_2)
        (`|ExecutionSequence`
          (:`then_0`
            (`KismetSystemLibrary.Delay` 0.2)
            (`SceneComponent.K2_SetWorldLocation` _cube _object_origin false false)
            (`SceneComponent.K2_SetWorldLocation` _item_sprite _object_origin false false))
          (:`then_1`
            (`SceneComponent.ToggleVisibility` (`self.Item_Sprite`) false :!label _label_3)))))
    (:`B`
      (if _returnvalue
        (`SceneComponent.K2_SetWorldLocation` _cube (0.0 1000.0 0.0) false false :!label _label_4)
        (goto _label_3)))))

(event `UnhideDrawerItems`
  (bind _returnvalue (and (not (`self.MouseOver`)) (`.CupboardItems` (`self.ItemsInStorage`))))
  (`/Engine/EditorBlueprintResources/StandardMacros.FlipFlop`
    (:`A`
      (if _returnvalue
        (goto _label_2)))
    (:`B`
      (if _returnvalue
        (goto _label_4)))))

(event `self.ReceiveTick`
  (params (DeltaSeconds :type "Float (single-precision)"))
  (bind _cube (`self.Cube`))
  (bind _cube_2 (`self.Cube`))
  (bind _worldlocation (`PlayerController.DeprojectMousePositionToWorld` (`GameplayStatics.GetPlayerController` 0)))
  (bind _returnvalue (`PlayerCameraManager.GetCameraLocation` (`GameplayStatics.GetPlayerCameraManager` 0)))
  (bind _returnvalue_x (`KismetMathLibrary.BreakVector` (`SceneComponent.K2_GetComponentLocation` _cube)))
  (`|ExecutionSequence`
    (:`then_1`
      ; move object with mouse
      (if (`self.bIsDragging`)
        (`SceneComponent.K2_SetWorldLocation` _cube (`KismetMathLibrary.MakeVector` _returnvalue_x (.y _worldlocation) (.z _worldlocation)) false false)))
    (:`then_2`
      ; Inspect Mode
      (if (and (`PlayerController.WasInputKeyJustPressed` (`GameplayStatics.GetPlayerController` 0) "RightMouseButton") (`self.MouseOver`) (not (`self.bIsDragging`)))
        (if (`self.Inspecting`)
          (set `self.Inspecting` false)
          (`SceneComponent.K2_SetWorldLocation` (`self.Cube`) (`self.Object Origin`) false false)
          (`self.K2_DestroyActor` (stale _returnvalue_2))
          (else
            (`SceneComponent.K2_SetWorldLocation` _cube_2 (+ _returnvalue (50.0 0.0 0.0)) false false)
            (`SceneComponent.SetRelativeScale3D` _cube_2 (2.0 2.0 2.0))
            (set `self.Inspecting` true)
            (bind _returnvalue_2 (`|SpawnActorFromClass` "/Game/Blueprint/Actors/THE_WALL.THE_WALL_C" (`KismetMathLibrary.MakeTransform` (+ _returnvalue (100.0 0.0 0.0))) "Undefined" "MultiplyWithRoot" null null))))))))

(event `self.Cube.OnReleased`
  (params (TouchedComponent :type "PrimitiveComponent Object Reference") (ButtonReleased :type "Key Structure"))
  (bind (_frideitems _cupboarditems) (`self.ItemsInStorage`))
  (bind _cube (`self.Cube`))
  (bind _endstubutref (`self.EndStuButRef`))
  (bind _tutref (`self.TutRef`))
  (bind _cure (`self.Cure`))
  ; object back to origin
  (if (`self.bIsDragging`)
    (if (not (`self.Inspecting`))
      (`|ExecutionSequence`
        (:`then_0`
          ; Execute the child
          (if (`self.OverChild`)
            (if (`/Game/Blueprint/Actors/BP_Prinicipal.TutorialActive` _tutref)
              (if (or (`KismetStringLibrary.EqualEqual_StrStr` _cure "Unholy Water") (`KismetStringLibrary.EqualEqual_StrStr` _cure "Holy Water") (`KismetStringLibrary.EqualEqual_StrStr` _cure "Water Bucket"))
                (`/Game/Blueprint/Actors/BP_Prinicipal.WaterGivenEvent` _tutref)
                (else
                  (`/Game/Blueprint/Actors/BP_Prinicipal.NotWaterGivenEvent` _tutref)))
              (else
                (bind _asbp_student (cast `/Game/Blueprint/Actors/BP_Student` (`self.student ref`)))
                (if (`KismetStringLibrary.EqualEqual_StrStr` (`self.Cure`) (`/Game/Blueprint/Actors/BP_Student.Current Cure` _asbp_student))
                  (set `/Game/Blueprint/Actors/BP_EndStubuttons.CureRight` true _endstubutref)
                  (`KismetSystemLibrary.PrintString` "CURED")
                  (else
                    (set `/Game/Blueprint/Actors/BP_EndStubuttons.CureRight` false _endstubutref)
                    (`KismetSystemLibrary.PrintString` "boowamp")))))))
        (:`then_1`
          (set `self.bIsDragging` false)
          (`SceneComponent.K2_SetWorldLocation` _cube (`self.Object Origin`) false false)
          (set `self.AtOrigin` true)
          (if (or _frideitems _cupboarditems)
            (`SceneComponent.SetVisibility` (`self.Item_Sprite`) false false)
            (`SceneComponent.K2_SetWorldLocation` _cube (0.0 1000.0 0.0) false false)
            (`self.SetActorTickEnabled` false)))))))

(event `self.ReceiveActorBeginOverlap`
  (params (OtherActor :type "Actor Object Reference"))
  ; overlapping child
  (`|ExecutionSequence`
    (:`then_0`
      (bind _asbp_student (cast `/Game/Blueprint/Actors/BP_Student` OtherActor))
      (set `self.OverChild` true)
      (set `self.student ref` _asbp_student))
    (:`then_1`
      (cast `/Game/Blueprint/Actors/BP_Prinicipal` OtherActor)
      (set `self.OverChild` true))))

(event `self.ReceiveActorEndOverlap`
  (params (OtherActor :type "Actor Object Reference"))
  ; overlapping child
  (`|ExecutionSequence`
    (:`then_0`
      (cast `/Game/Blueprint/Actors/BP_Student` OtherActor)
      (set `self.OverChild` false))
    (:`then_1`
      (cast `/Game/Blueprint/Actors/BP_Prinicipal` OtherActor)
      (set `self.OverChild` false))))

(fn `UserConstructionScript`)