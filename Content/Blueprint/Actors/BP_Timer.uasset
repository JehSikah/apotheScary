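; BP_Timer is a countdown clock actor that, on expiry, broadcasts completion, spawns THE_WALL at an offset from the player camera and plays a school bell.
; TimerStart sets a per-second timer that decrements a Timespan and, once only, runs a timeline rotating the hour hand through a full turn.
; Tick polls for a zero Timespan and fires the completion logic through a DoOnce that resets while time remains.
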(event `self.ReceiveBeginPlay`
  (set `self.Timer Go` true)
  (set `self.StartingPos` (struct))
  (set `self.EndPos` (struct :`Pitch` -360.0)))

(event `Timer Start`
  (`KismetSystemLibrary.K2_SetTimer` null "TimerTickDown" 1.0 (`self.Timer Go`))
  (`/Engine/EditorBlueprintResources/StandardMacros.DoOnce` false
    (:`Completed`
      (bind (_direction _hourhand) (`Timeline|RotateHand` :!via `PlayFromStart`)
        (:`Update`
          (`SceneComponent.K2_SetRelativeRotation` (`self.HourHand`) (`KismetMathLibrary.RLerp` (`self.StartingPos`) (`self.EndPos`) _hourhand) false false))))))

(event `self.ReceiveTick`
  (params (DeltaSeconds :type "Float (single-precision)"))
  (if (== (`self.timespan`) (`KismetMathLibrary.TimespanZeroValue`))
    (`/Engine/EditorBlueprintResources/StandardMacros.DoOnce` false :!label _label
      (:`Completed`
        (set `self.Timer Go` false)
        (`self.TimerCompleted`)
        (`|SpawnActorFromClass` "/Game/Blueprint/Actors/THE_WALL.THE_WALL_C" (`KismetMathLibrary.MakeTransform` (+ (`PlayerCameraManager.GetCameraLocation` (`GameplayStatics.GetPlayerCameraManager` 0)) (100.0 0.0 0.0))) "Undefined" "MultiplyWithRoot" null null)
        (`GameplayStatics.PlaySound2D` "/Game/Sounds/SchoolBell.SchoolBell" 1.0 1.0 0.0 null null)))
    (else
      (goto _label :!via `Reset`))))

(fn `TimerTickDown`
  (if (not (== (stale _output_get) (`KismetMathLibrary.TimespanZeroValue`)))
    (bind _output_get (set `self.timespan` (- (`self.timespan`) (`KismetMathLibrary.MakeTimespan2` 0 0 0 1))))))

(fn `UserConstructionScript`)