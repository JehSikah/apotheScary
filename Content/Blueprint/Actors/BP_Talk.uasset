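; BP_Talk is an actor with a TalkText component, apparently a talk indicator tied to BP_Student, that currently stays hidden.
; BeginPlay hides TalkText and looks up a BP_Student, and Tick is empty.
; Disconnected leftover logic would toggle the text through the student's SpawnFinished and EventCured or its diagnosing and movement flags, with debug prints, but none of it runs.
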(event `self.ReceiveTick`
  (params (DeltaSeconds :type "Float (single-precision)")))

(event `self.ReceiveBeginPlay`
  (`SceneComponent.SetVisibility` (`self.TalkText`) false false)
  (bind _returnvalue (`GameplayStatics.GetActorOfClass` "/Game/Blueprint/Actors/BP_Student.BP_Student_C")))

(fn `UserConstructionScript`)