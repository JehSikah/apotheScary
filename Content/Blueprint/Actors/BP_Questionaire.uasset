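; Questionnaire actor that picks the three answers a student patient gives, based on species, disease and whether they are faking.
; On BeginPlay it caches the managers and student, binds to the spawn-finish event, and copies both answer DataTables into arrays, with the faker load nested inside the student loop.
; On spawn, fakers read a per-species map in the first faker row; others use a species-offset-plus-disease row, both indexed by StudentEntranceInt.
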(event `self.ReceiveBeginPlay`
  (bind _dt_studentanswersref (`self.DT_StudentAnswersRef`))
  (bind _dt_fakeranswersref (`self.DT_FakerAnswersRef`))
  (`self.EnableInput` (`GameplayStatics.GetPlayerController` 0))
  (bind _returnvalue (`GameplayStatics.GetActorOfClass` "/Game/Blueprint/Actors/BP_CureObjects.BP_CureObjects_C"))
  (set `self.setobj` _returnvalue)
  (bind _outactors (`GameplayStatics.GetAllActorsOfClass` "/Game/Blueprint/Actors/BP_DialogueManager.BP_DialogueManager_C"))
  (set `self.DialogueMan` (`|GetArrayItem` _outactors))
  (bind _returnvalue_2 (`GameplayStatics.GetActorOfClass` "/Game/Blueprint/Actors/BP_Student.BP_Student_C"))
  (bind _output_get (set `self.StudentReff` _returnvalue_2))
  (add `/Game/Blueprint/Actors/BP_Student.SpawnFinishDispatch` _output_get (delegate `StudentSpawned`))
  (bind _outactors_2 (`GameplayStatics.GetAllActorsOfClass` "/Game/Blueprint/Actors/BP_DiseaseManager.BP_DiseaseManager_C"))
  (set `self.DeseaseManagerRef` (`|GetArrayItem` _outactors_2))
  (bind _outrownames (`DataTableFunctionLibrary.GetDataTableRowNames` _dt_studentanswersref))
  (for _array_element _outrownames
    (bind _returnvalue_3 (`|GetDataTableRow` _dt_studentanswersref _array_element)
      (:`then`
        (`KismetArrayLibrary.Array_Add` (`self.STR_StudentAnswersRef`) _returnvalue_3)
        (bind _outrownames_2 (`DataTableFunctionLibrary.GetDataTableRowNames` _dt_fakeranswersref))
        (for _array_element_2 _outrownames_2
          (bind _returnvalue_4 (`|GetDataTableRow` _dt_fakeranswersref _array_element_2)
            (:`then`
              (`KismetArrayLibrary.Array_Add` (`self.STR_FalerAnswersRef`) _returnvalue_4))))))))

(event `StudentSpawned`
  (bind _studententranceint (`/Game/Blueprint/Actors/BP_DialogueManager.StudentEntranceInt` (`self.DialogueMan`)))
  (bind _studentrefenum (`/Game/Blueprint/Actors/BP_Student.StudentRefEnum` (`self.StudentReff`)))
  (bind (_disease _student _howlong _where _q3) (break `/Game/Blueprint/Data-Structs/StudentAnswers/STR_StudentAnswers` (`|GetArrayItem` (`self.STR_StudentAnswersRef`) (`self.StuSeaseRow`))))
  (bind (_introdialogue _howlong_2 _where_2 _fakeanswer3) (break `/Game/Blueprint/Data-Structs/StudentAnswers/STR_FakerStrings` (`BlueprintMapLibrary.Map_Find` (`.NumeratorMap_13_34E03E844849F4B2DD6C45B748DF2924` (break `/Game/Blueprint/Data-Structs/StudentAnswers/STR_FakerAnswers` (`|GetArrayItem` (`self.STR_FalerAnswersRef`)))) _studentrefenum)))
  (if (`/Game/Blueprint/Actors/BP_DiseaseManager.Faker` (`self.DeseaseManagerRef`))
    (set `self.Answer1` (`|GetArrayItem` _howlong_2 _studententranceint))
    (set `self.Answer2` (`|GetArrayItem` _where_2 _studententranceint))
    (set `self.Answer3` (`|GetArrayItem` _fakeanswer3 _studententranceint))
    (else
      (switch `/Game/Blueprint/Data-Structs/Enums/StudentType` _studentrefenum
        (:`NewEnumerator0`
          ; Mini Machine
          (`self.SetStuSeaseRow` 0))
        (:`NewEnumerator1`
          (`self.SetStuSeaseRow` 13))
        (:`NewEnumerator2`
          (`self.SetStuSeaseRow` 26))
        (:`NewEnumerator3`
          (`self.SetStuSeaseRow` 39))
        (:`NewEnumerator4`
          (`self.SetStuSeaseRow` 52))
        (:`NewEnumerator5`
          (`self.SetStuSeaseRow` 65))
        (:`NewEnumerator6`
          (`self.SetStuSeaseRow` 78))
        (:`NewEnumerator7`
          (`self.SetStuSeaseRow` 91))
        (:`NewEnumerator8`
          (`self.SetStuSeaseRow` 104)))
      (set `self.Answer1` (`|GetArrayItem` _howlong _studententranceint))
      (set `self.Answer2` (`|GetArrayItem` _where _studententranceint))
      (set `self.Answer3` (`|GetArrayItem` _q3 _studententranceint))
      (if true
        _))))

(fn `SetStuSeaseRow`
  (params (`add one in` :type Integer))
  (returns (`add one out` :type Integer))
  (switch `/Game/Blueprint/Data-Structs/Enums/Enum_DiseaseType` (`/Game/Blueprint/Actors/BP_DiseaseManager.Disease Enum` (`self.DeseaseManagerRef`))
    (:`NewEnumerator0`
      (set `self.StuSeaseRow` `add one in`))
    (:`NewEnumerator1`
      (set `self.StuSeaseRow` (+ `add one in` 1)))
    (:`NewEnumerator2`
      (set `self.StuSeaseRow` (+ `add one in` 2)))
    (:`NewEnumerator3`
      (set `self.StuSeaseRow` (+ `add one in` 3)))
    (:`NewEnumerator4`
      (set `self.StuSeaseRow` (+ `add one in` 4)))
    (:`NewEnumerator7`
      (set `self.StuSeaseRow` (+ `add one in` 5)))
    (:`NewEnumerator8`
      (set `self.StuSeaseRow` (+ `add one in` 6)))
    (:`NewEnumerator9`
      (set `self.StuSeaseRow` (+ `add one in` 7)))
    (:`NewEnumerator10`
      (set `self.StuSeaseRow` (+ `add one in` 8)))
    (:`NewEnumerator11`
      (set `self.StuSeaseRow` (+ `add one in` 9)))
    (:`NewEnumerator12`
      (set `self.StuSeaseRow` (+ `add one in` 10)))
    (:`NewEnumerator13`
      (set `self.StuSeaseRow` (+ `add one in` 11)))
    (:`NewEnumerator15`
      (set `self.StuSeaseRow` (+ `add one in` 12))))
  (return 0))

(fn `UserConstructionScript`)