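; Tutorial actor that brings the school principal (TheBigMan) on and off screen to introduce levels in a school nurse game.
; It binds to BP_Levels' game-start and new-level events, also triggering itself on BeginPlay when LevelNum isn't 1.
; The principal slides in and fires CallPrincipalEvent, while PrincipalLeave slides him out, hides him and fires CallPrincipalOverEvent.
; The tutorial dialogue, level switch and flipbook nodes are disconnected and never run.
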(event `self.ReceiveBeginPlay`
  (bind _returnvalue (`GameplayStatics.GetActorOfClass` "/Game/Blueprint/Actors/BP_Levels.BP_Levels_C"))
  (bind _output_get (set `self.LevelsRef` _returnvalue))
  (add `/Game/Blueprint/Actors/BP_Levels.GameStart` _output_get (delegate `NewGamePressed`))
  (add `/Game/Blueprint/Actors/BP_Levels.NewLevel` _output_get (delegate `NewLevel`))
  (bind _asbp_game_instance (cast `/Game/Blueprint/BP_GameInstance` (`GameplayStatics.GetGameInstance`)))
  (bind _output_get_2 (set `self.As BP Game Instance` _asbp_game_instance))
  (bind _output_get_3 (set `self.TutLevelNum` (`/Game/Blueprint/BP_GameInstance.LevelNum` _output_get_2)))
  (if (!= _output_get_3 1)
    (`self.NewLevel`)))

(event `NewGamePressed`
  (bind _thebigman (`self.TheBigMan`))
  (set `self.TutorialActive` true :!label _label)
  (`KismetSystemLibrary.Delay` 1.0)
  (`SceneComponent.SetVisibility` _thebigman true false)
  (set `self.TutLevelNum` (`/Game/Blueprint/BP_GameInstance.LevelNum` (stale `self.ReceiveBeginPlay` _asbp_game_instance)))
  (`KismetSystemLibrary.MoveComponentTo` _thebigman (400.0 -250.0 90.0) (struct :`Yaw` -90.0) true false 1.0)
  (`self.PrincipalEvent`))

(event `NewLevel`
  (goto _label))

(event `PrincipalLeave`
  (bind _thebigman (`self.TheBigMan`))
  (`KismetSystemLibrary.MoveComponentTo` _thebigman (400.0 -800.0 90.0) (struct) false true 1.0)
  (`SceneComponent.SetVisibility` _thebigman false false)
  (set `self.TutorialActive` false)
  (`self.PrincipalOverEvent`))

(fn `UserConstructionScript`)