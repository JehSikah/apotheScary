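; BP_PooledActor is an object pool actor that switches between in-use and dormant states rather than being destroyed.
; It starts dormant on BeginPlay, and SetInUse toggles its collision, visibility and tick together.
; Activation starts a timer of StudentPerish length that fires StudentCured, which returns the actor to dormant.
; Each SetInUse call clears any pending timer first.
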(event `self.ReceiveBeginPlay`
  (`self.SetInUse` false))

(event `SetInUse`
  (params (inUse :type Boolean))
  (set `self.inUse` inUse)
  (`self.SetActorEnableCollision` inUse)
  (`self.SetActorHiddenInGame` (not inUse))
  (`self.SetActorTickEnabled` inUse)
  (`KismetSystemLibrary.K2_ClearAndInvalidateTimerHandle` (`self.TimeToPerishTimer`))
  (if inUse
    (bind _returnvalue (`KismetSystemLibrary.K2_SetTimerDelegate` (delegate `StudentCured`) (`self.StudentPerish`)))
    (set `self.TimeToPerishTimer` _returnvalue)))

(event `StudentCured`
  (`self.SetInUse` false))

(fn `UserConstructionScript`)