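; BP_Storage is a clickable storage actor with a fridge and a drawer cupboard that open and close on click.
; Clicks on each box toggle its open/closed flipbook and play door sounds, first closing the other unit if it is open.
; Each state change fires the OpeningFridge or OpeningDrawer call.
; Opening the fridge also spawns an old-refrigerator sound, which is toggled via ToggleActive on closing.
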(event `self.ReceiveBeginPlay`)

(event `self.Drawersbox.OnClicked`
  (params (TouchedComponent :type "PrimitiveComponent Object Reference") (ButtonPressed :type "Key Structure"))
  (bind _drawers (`self.Drawers`))
  (if (`self.FridgeOpen`)
    (`PaperFlipbookComponent.SetFlipbook` (`self.Fridge`) "/Game/VisualAssets/WorldSprites/FB_FridgeClosed.FB_FridgeClosed")
    (`self.OpeningFridge`)
    (set `self.FridgeOpen` false)
    (`GameplayStatics.PlaySound2D` "/Game/Sounds/FridgeClosesound.FridgeClosesound" 1.0 1.0 0.0 null null)
    (`ActorComponent.ToggleActive` (stale _returnvalue)))
  (if (`self.CupboardOpen`)
    (`PaperFlipbookComponent.SetFlipbook` _drawers "/Game/VisualAssets/WorldSprites/FB_CupboardClosed.FB_CupboardClosed")
    (`self.OpeningDrawer`)
    (set `self.CupboardOpen` false)
    (`GameplayStatics.PlaySound2D` "/Game/Sounds/doorclosingsound.doorclosingsound" 1.0 1.0 0.0 null null)
    (else
      (`PaperFlipbookComponent.SetFlipbook` _drawers "/Game/VisualAssets/WorldSprites/FB_CupboardOpen.FB_CupboardOpen")
      (`self.OpeningDrawer`)
      (set `self.CupboardOpen` true)
      (`GameplayStatics.PlaySound2D` "/Game/Sounds/dooropensound.dooropensound" 1.0 1.0 0.0 null null))))

(event `self.FridgeBox.OnClicked`
  (params (TouchedComponent :type "PrimitiveComponent Object Reference") (ButtonPressed :type "Key Structure"))
  (bind _fridge (`self.Fridge`))
  (if (`self.CupboardOpen`)
    (`PaperFlipbookComponent.SetFlipbook` (`self.Drawers`) "/Game/VisualAssets/WorldSprites/FB_CupboardClosed.FB_CupboardClosed")
    (`self.OpeningDrawer`)
    (set `self.CupboardOpen` false)
    (`GameplayStatics.PlaySound2D` "/Game/Sounds/doorclosingsound.doorclosingsound" 1.0 1.0 0.0 null null))
  (if (`self.FridgeOpen`)
    (`PaperFlipbookComponent.SetFlipbook` _fridge "/Game/VisualAssets/WorldSprites/FB_FridgeClosed.FB_FridgeClosed")
    (`self.OpeningFridge`)
    (set `self.FridgeOpen` false)
    (`GameplayStatics.PlaySound2D` "/Game/Sounds/FridgeClosesound.FridgeClosesound" 1.0 1.0 0.0 null null)
    (`ActorComponent.ToggleActive` (stale _returnvalue))
    (else
      (`PaperFlipbookComponent.SetFlipbook` _fridge "/Game/VisualAssets/WorldSprites/FB_FridgeOpen.FB_FridgeOpen")
      (`self.OpeningFridge`)
      (set `self.FridgeOpen` true)
      (`GameplayStatics.PlaySound2D` "/Game/Sounds/Fridge_Open.Fridge_Open" 1.0 1.0 0.0 null null)
      (bind _returnvalue (`GameplayStatics.SpawnSound2D` "/Game/Sounds/the-sound-of-an-old-refrigerator-137492.the-sound-of-an-old-refrigerator-137492" 1.0 1.0 0.0 null)))))

(fn `UserConstructionScript`)