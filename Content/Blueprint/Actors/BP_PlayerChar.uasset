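; Player character for a mouse-driven game, owning the camera movement, UI widgets and pause menu.
; Hovering Uppies or Downies runs timelines sliding the capsule between two heights, toggling tutorial or history UI.
; BeginPlay creates every widget, enables cursor events and binds BP_Timer completion to hide gameplay panels.
; Pause flip-flops menus and spawns THE_WALL before the camera, but unpauses and destroys it only while BP_Principal's tutorial is active.
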(event `self.uppies.OnBeginCursorOver`
  (params (TouchedComponent :type "PrimitiveComponent Object Reference"))
  (bind _top_location (`self.Top_Location`))
  ; Move yor ass
  (if (not (`self.Top_Screen`))
    (bind (_direction _newtrack_2) (`Timeline|Move speed two` :!via `PlayFromStart`)
      (:`Update`
        (`SceneComponent.K2_SetWorldLocation` (`self.CapsuleComponent`) (`KismetMathLibrary.VLerp` (- _top_location (0.0 0.0 280.0)) _top_location _newtrack_2) false false)
        (set `self.Top_Screen` true)
        (if (`/Game/Blueprint/Actors/BP_Principal.TutorialActive` (`self.TutorialRef`))
          (`Widget.SetVisibility` (`self.TutorialUI`) "SelfHitTestInvisible")
          (else
            (`Widget.SetVisibility` (`self.History UI`) "SelfHitTestInvisible")))))))

(event `self.downies.OnBeginCursorOver`
  (params (TouchedComponent :type "PrimitiveComponent Object Reference"))
  (bind _top_location (`self.Top_Location`))
  ; Move yor ass
  (if (`self.Top_Screen`)
    (`Widget.SetVisibility` (`self.TutorialUI`) "Hidden")
    (`Widget.SetVisibility` (`self.History UI`) "Hidden")
    (bind (_direction _newtrack_2) (`Timeline|move speed` :!via `PlayFromStart`)
      (:`Update`
        (`SceneComponent.K2_SetWorldLocation` (`self.CapsuleComponent`) (`KismetMathLibrary.VLerp` _top_location (- _top_location (0.0 0.0 280.0)) _newtrack_2) false false)
        (set `self.Top_Screen` false)))))

(event `self.ReceiveTick`
  (params (DeltaSeconds :type "Float (single-precision)")))

(event `self.ReceiveBeginPlay`
  (bind _returnvalue (`GameplayStatics.GetPlayerController` 0))
  (bind _asbp_game_instance (cast `/Game/Blueprint/BP_GameInstance` (`GameplayStatics.GetGameInstance`)))
  (bind _returnvalue_2 (`GameplayStatics.GetActorOfClass` "/Game/Blueprint/Actors/BP_Timer.BP_Timer_C"))
  (bind _output_get (set `self.TimerRef` _returnvalue_2))
  (add `/Game/Blueprint/Actors/BP_Timer.TimerCompleted` _output_get (delegate `HideStuff`))
  (bind _returnvalue_3 (`GameplayStatics.GetActorOfClass` "/Game/Blueprint/Actors/BP_Principal.BP_Principal_C"))
  (bind _output_get_2 (set `self.TutorialRef` _returnvalue_3))
  (add `/Game/Blueprint/Actors/BP_Principal.PrincipalOverEvent` _output_get_2 (delegate `WIDGETS PLEASe`))
  ; UI Set Up
  (bind _returnvalue_4 (`|CreateWidget` "/Game/Blueprint/Wijit/WB_MainMenu.WB_MainMenu_C"))
  (bind _output_get_3 (set `self.MainMenuUI` _returnvalue_4))
  (`UserWidget.AddToViewport` _output_get_3 0)
  (if (== (`/Game/Blueprint/BP_GameInstance.LevelNum` _asbp_game_instance) 0)
    (`Widget.SetVisibility` _output_get_3 "Visible")
    (else
      (`Widget.SetVisibility` _output_get_3 "Hidden")))
  (bind _returnvalue_5 (`|CreateWidget` "/Game/Blueprint/Wijit/WB_Options.WB_Options_C"))
  (bind _output_get_4 (set `self.OptionsUI` _returnvalue_5))
  (`UserWidget.AddToViewport` _output_get_4 0)
  (`Widget.SetVisibility` _output_get_4 "Hidden")
  (bind _returnvalue_6 (`|CreateWidget` "/Game/Blueprint/Wijit/WB_TutorialText.WB_TutorialText_C"))
  (bind _output_get_5 (set `self.TutorialUI` _returnvalue_6))
  (`UserWidget.AddToViewport` _output_get_5 0)
  (`Widget.SetVisibility` _output_get_5 "Hidden")
  (bind _returnvalue_7 (`|CreateWidget` "/Game/Blueprint/Wijit/WB_History.WB_History_C"))
  (bind _output_get_6 (set `self.History UI` _returnvalue_7))
  (`UserWidget.AddToViewport` _output_get_6 0)
  (`Widget.SetVisibility` _output_get_6 "Hidden")
  (bind _returnvalue_8 (`|CreateWidget` "/Game/Blueprint/Wijit/WB_BookUI.WB_BookUI_C"))
  (bind _output_get_7 (set `self.BookUI` _returnvalue_8))
  (`UserWidget.AddToViewport` _output_get_7 0)
  (`Widget.SetVisibility` _output_get_7 "Hidden")
  (bind _returnvalue_9 (`|CreateWidget` "/Game/Blueprint/Wijit/WB_Pause.WB_Pause_C"))
  (bind _output_get_8 (set `self.PauseUI` _returnvalue_9))
  (`UserWidget.AddToViewport` _output_get_8 0)
  (`Widget.SetVisibility` _output_get_8 "Hidden")
  (bind _returnvalue_10 (`|CreateWidget` "/Game/Blueprint/Wijit/WB_Diagnose.WB_Diagnose_C"))
  (bind _output_get_9 (set `self.Diagnose UI` _returnvalue_10))
  (`UserWidget.AddToViewport` _output_get_9 0)
  (`Widget.SetVisibility` _output_get_9 "Hidden")
  (bind _returnvalue_11 (`|CreateWidget` "/Game/Blueprint/Wijit/WB_EndLevel.WB_EndLevel_C"))
  (bind _output_get_10 (set `self.EndLevelUI` _returnvalue_11))
  (`UserWidget.AddToViewport` _output_get_10 0)
  (`Widget.SetVisibility` _output_get_10 "Hidden")
  ; the sequence machine
  (`|ExecutionSequence`
    (:`then_0`
      (set `PlayerController.bEnableClickEvents` true _returnvalue)
      (`EnhancedInputSubsystemInterface.AddMappingContext` (pcsubsystem `EnhancedInputLocalPlayerSubsystem` _returnvalue) "/Game/Inputs/INP_Context.INP_Context" 0 (struct) :!label _label))
    (:`then_1`
      (set `PlayerController.bEnableMouseOverEvents` true _returnvalue)
      (goto _label))
    (:`then_2`
      (set `PlayerController.bShowMouseCursor` true _returnvalue)
      (goto _label))
    (:`then_3`
      ; set origin
      (set `self.Top_Location` (`SceneComponent.K2_GetComponentLocation` (`self.CapsuleComponent`)))
      (set `self.Top_Screen` true))))

(event `EnhancedInput|/Game/Inputs/INP_Look`
  (params (ActionValue :type "Vector2D Structure") (ElapsedSeconds :type "Float (double-precision)") (TriggeredSeconds :type "Float (double-precision)") (InputAction :type "InputAction Object Reference" :default "/Game/Inputs/INP_Look.INP_Look"))
  (bind _returnvalue (`GameplayStatics.GetPlayerCameraManager` 0))
  (:`Triggered`
    (`self.AddControllerYawInput` ActionValue_X)
    (`self.AddControllerPitchInput` ActionValue_Y)
    ;[0.05821 0.15 0.0439 0.5] Sets constrains for the camera on BeginPlay
    (set `PlayerCameraManager.ViewPitchMax` 10.0 _returnvalue)
    (set `PlayerCameraManager.ViewPitchMin` -45.0 _returnvalue)
    (set `PlayerCameraManager.ViewYawMax` 0.0 _returnvalue)
    (set `PlayerCameraManager.ViewYawMin` 0.0 _returnvalue)))

(event `HideStuff`
  (`Widget.SetVisibility` (`self.BookUI`) "Hidden")
  (`Widget.SetVisibility` (`self.Diagnose UI`) "Hidden")
  (`Widget.SetVisibility` (`self.History UI`) "Hidden"))

(event `self.ReceiveActorBeginCursorOver`)

(event `WIDGETS PLEASe`)

(event `EnhancedInput|/Game/Inputs/INP_Pause`
  (params (ActionValue :type Boolean) (ElapsedSeconds :type "Float (double-precision)") (TriggeredSeconds :type "Float (double-precision)") (InputAction :type "InputAction Object Reference" :default "/Game/Inputs/INP_Pause.INP_Pause"))
  (bind _history_ui (`self.History UI`))
  (bind _pauseui (`self.PauseUI`))
  (bind _endlevelui (`self.EndLevelUI`))
  ; Pause Menu
  (:`Started`
    (`/Engine/EditorBlueprintResources/StandardMacros.FlipFlop`
      (:`A`
        (set `self.IsPaused` true)
        (`Widget.SetVisibility` _history_ui "Hidden")
        (`Widget.SetVisibility` _endlevelui "Hidden")
        (`Widget.SetVisibility` _pauseui "Visible")
        (bind _returnvalue (`|SpawnActorFromClass` "/Game/Blueprint/Actors/THE_WALL.THE_WALL_C" (`KismetMathLibrary.MakeTransform` (+ (`PlayerCameraManager.GetCameraLocation` (`GameplayStatics.GetPlayerCameraManager` 0)) (100.0 0.0 0.0))) "Undefined" "MultiplyWithRoot" null null))
        (`GameplayStatics.SetGamePaused` true))
      (:`B`
        (set `self.IsPaused` false)
        (`Widget.SetVisibility` _pauseui "Hidden")
        (if (`/Game/Blueprint/Actors/BP_Timer.Timer Go` (`self.TimerRef`))
          (`Widget.SetVisibility` _endlevelui "Hidden")
          (else
            (`Widget.SetVisibility` _endlevelui "Visible")))
        (if (`/Game/Blueprint/Actors/BP_Principal.TutorialActive` (`self.TutorialRef`))
          (`Widget.SetVisibility` _history_ui "Hidden")
          (`self.K2_DestroyActor` _returnvalue)
          (`GameplayStatics.SetGamePaused` false)
          (else
            (`Widget.SetVisibility` _history_ui "SelfHitTestInvisible")))))))

(fn `Hunterscoolfuncteiop`
  (params (Bbject :type "/Game/Blueprint/Actors/BP_CureObjects Object Reference"))
  (`KismetSystemLibrary.PrintString` (`KismetSystemLibrary.GetDisplayName` Bbject)))

(fn `UserConstructionScript`)