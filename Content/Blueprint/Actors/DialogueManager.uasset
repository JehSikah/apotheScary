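; DialogueManager picks the line a student speaks about their illness once the student finishes spawning.
; On BeginPlay it finds BP_DiseaseManager and BP_Student and binds to the student's SpawnFinish dispatcher.
; For real diseases, it splits the student type's first-symptom string on "$" into three variants, picks one randomly and calls CallTextSet.
; The unfinished faker branch only joins fake disease and student type into CastText, without that call.
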(event `CustomEvent`
  (bind _student_refer (`self.Student Refer`))
  (bind _diseasemanagerref (`self.DiseaseManagerRef`))
  (bind _studenttypestring (break `/Game/Blueprint/Data-Structs/STR_StudentInfo` (`|GetArrayItem` (`/Game/Blueprint/Actors/BP_Student.StudentType` _student_refer) (`/Game/Blueprint/Actors/BP_Student.StudentRowPick` _student_refer))))
  (bind (_lefts _rights) (`KismetStringLibrary.Split` (`BlueprintMapLibrary.Map_Find` (`.Sympt1_Syntax_31_48E66F054BBFA9C92702F7B49A38B7F0` (break `/Game/Blueprint/Data-Structs/STR_Disease` (`|GetArrayItem` (`/Game/Blueprint/Actors/BP_DiseaseManager.DiseaseStrRef` _diseasemanagerref) (`/Game/Blueprint/Actors/BP_DiseaseManager.DiseaseRowPick` _diseasemanagerref)))) _studenttypestring) "$"))
  (bind (_lefts_2 _rights_2) (`KismetStringLibrary.Split` _rights "$"))
  (bind _array (`|MakeArray` _lefts _lefts_2 _rights_2))
  (if (`/Game/Blueprint/Actors/BP_DiseaseManager.Faker` _diseasemanagerref)
    ; also this does basically nothing right now
    ;; change to state machine to decide students speech / how a student answers to questions.
    (set `self.CastText` (`KismetTextLibrary.Conv_StringToText` (`KismetStringLibrary.Concat_StrStr` (`.FakeDisease_2_E315DBC5432C186BCDC17D8B635F0B72` (break `/Game/Blueprint/Data-Structs/STR_Faker` (`|GetArrayItem` (`/Game/Blueprint/Actors/BP_DiseaseManager.Faker STR Ref` _diseasemanagerref) (`/Game/Blueprint/Actors/BP_DiseaseManager.Faker Row Pick` _diseasemanagerref)))) (`|GetEnumeratorNameAsString` _studenttypestring))))
    (else
      (set `self.StudentEntranceInt` (`KismetMathLibrary.RandomInteger` (`KismetArrayLibrary.Array_Length` _array)))
      (set `self.CastText` (`|GenericToText` (`|GetArrayItem` _array (`self.StudentEntranceInt`))))
      (`self.TextSet`))))

(event `self.ReceiveBeginPlay`
  (bind _outactors (`GameplayStatics.GetAllActorsOfClass` "/Game/Blueprint/Actors/BP_DiseaseManager.BP_DiseaseManager_C"))
  (set `self.DiseaseManagerRef` (`|GetArrayItem` _outactors))
  (cast `/Game/Blueprint/Actors/BP_DiseaseManager` (`self.DiseaseManagerRef`))
  (bind _outactors_2 (`GameplayStatics.GetAllActorsOfClass` "/Game/Blueprint/Actors/BP_Student.BP_Student_C"))
  (bind _output_get (set `self.Student Refer` (`|GetArrayItem` _outactors_2)))
  (bind _asbp_student (cast `/Game/Blueprint/Actors/BP_Student` _output_get))
  (add `/Game/Blueprint/Actors/BP_Student.SpawnFinishDispatch` _asbp_student (delegate `CustomEvent`)))

(fn `UserConstructionScript`)