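; Questionnaire actor that picks a student's row of answers from the student's monster type and the current disease.
; BeginPlay loads the answer data table into an array and binds to the first BP_Student's spawn-finish dispatcher.
; That event calls SetStuSeaseRow, chaining outputs across mutually exclusive type branches; only Hakkarian Blood Plague uses the input, other diseases increment the stored row.
; Debug key 8 prints the selected answers; older hard-coded row switches remain disconnected.
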(event Custom|CustomEvent
  (switch Utilities|FlowControl|Switch|SwitchonStudentType (Variables|/Game/Blueprint/Actors/BP_Student.BP_Student_C|GetStudentRefEnum (Variables|Default|GetStudentRef))
    (:NewEnumerator0
      ;[0.15 0.15 0.15 0.5] Mini Machine
      (bind _add_one_out (CallFunction|SetStuSeaseRow)))
    (:NewEnumerator1
      (bind _add_one_out_2 (CallFunction|SetStuSeaseRow _add_one_out)))
    (:NewEnumerator2
      (bind _add_one_out_3 (CallFunction|SetStuSeaseRow _add_one_out_2)))
    (:NewEnumerator3
      (bind _add_one_out_4 (CallFunction|SetStuSeaseRow _add_one_out_3)))
    (:NewEnumerator4
      (bind _add_one_out_5 (CallFunction|SetStuSeaseRow _add_one_out_4)))
    (:NewEnumerator5
      (CallFunction|SetStuSeaseRow _add_one_out_5))))

(event EventBeginPlay
  (bind _dt_studentanswersref (Variables|Default|GetDT_StudentAnswersRef))
  (Input|EnableInput (Game|GetPlayerController 0))
  (bind _outactors (Actor|GetAllActorsOfClass "/Game/Blueprint/Actors/BP_Student.BP_Student_C"))
  (bind _output_get (Variables|Default|SetStudentRef (Utilities|Array|Get(acopy) _outactors)))
  (EventDispatchers|BindEventtoSpawnFinishDispatch _output_get (delegate Custom|CustomEvent))
  (bind _outactors_2 (Actor|GetAllActorsOfClass "/Game/Blueprint/Actors/BP_DiseaseManager.BP_DiseaseManager_C"))
  (Variables|Default|SetDeseaseManagerRef (Utilities|Array|Get(acopy) _outactors_2))
  (bind _outrownames (DataTable|GetDataTableRowNames _dt_studentanswersref))
  (for _array_element _outrownames
    (bind _returnvalue (Utilities|GetDataTableRow _dt_studentanswersref _array_element)
      (:then
        (Utilities|Array|Add (Variables|Default|GetSTR_StudentAnswersRef) _returnvalue)))))

(event Collision|EventActorBeginOverlap
  (params (OtherActor :type Actor%20Object%20Reference)))

(event Input|KeyboardEvents|DebugKey8
  (params (Key :type Key%20Structure :default "None") (ActionValue :type Input%20Action%20Value%20Structure))
  (bind _str_studentanswersref (Variables|Default|GetSTR_StudentAnswersRef))
  (bind _stuseaserow (Variables|Default|GetStuSeaseRow))
  (bind _output (Utilities|Array|Get(acopy) _str_studentanswersref _stuseaserow))
  (bind (_disease _student _q1 _q2 _q3) (Utilities|Struct|BreakSTR_StudentAnswers _output))
  (:Pressed
    (Development|PrintString _q1)
    (Development|PrintString _q2)
    (Development|PrintString _q3)))

(fn ConstructionScript)

(fn SetStuSeaseRow
  (params (add%20one%20in :type Integer))
  (switch Utilities|FlowControl|Switch|SwitchonEnum_DiseaseType (Variables|/Game/Blueprint/Actors/BP_DiseaseManager.BP_DiseaseManager_C|GetDisease%20Enum (Variables|Default|GetDeseaseManagerRef))
    (:NewEnumerator0
      (bind _output_get (Variables|Default|SetStuSeaseRow add%20one%20in)))
    (:NewEnumerator1
      (bind _output_get_2 (Variables|Default|SetStuSeaseRow (+ _output_get 1))))
    (:NewEnumerator2
      (bind _output_get_3 (Variables|Default|SetStuSeaseRow (+ _output_get_2 1))))
    (:NewEnumerator3
      (bind _output_get_4 (Variables|Default|SetStuSeaseRow (+ _output_get_3 1))))
    (:NewEnumerator4
      (bind _output_get_5 (Variables|Default|SetStuSeaseRow (+ _output_get_4 1)))))
  (return (+ _output_get_5 1)))