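; Test actor for a draggable cure cube that cures a BP_Student when dragged onto one whose CurrentCure matches.
; BeginPlay stores its origin and loads the disease DataTable, taking its Cure from the CureNumber index.
; Hover enlarges the cube; click-hold drags it on Tick using deprojected mouse Y/Z with fixed X, and release snaps it back.
; Older line-trace drag experiments remain disconnected, and debug prints are left in.
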(event `CustomEvent` :!signature `self.OnClicked`
  (params (TouchedActor :type "Actor Object Reference") (ButtonPressed :type "Key Structure" :default "None")))

(event `self.ReceiveActorBeginOverlap`
  (params (OtherActor :type "Actor Object Reference"))
  (if (`self.bIsDragging`)
    (bind _asbp_student (cast `/Game/Blueprint/Actors/BP_Student` OtherActor))
    (if (`KismetStringLibrary.EqualEqual_StrStr` (`self.Cure`) (`/Game/Blueprint/Actors/BP_Student.Current Cure` _asbp_student))
      (`/Game/Blueprint/Actors/BP_Student.EventCured` _asbp_student)
      (else
        (`KismetSystemLibrary.PrintString` "boowamp")))))

(event `self.ReceiveBeginPlay`
  (bind _diseasetableref (`self.DiseaseTableRef`))
  ; find object starting point
  (set `self.Object Origin` (`self.K2_GetActorLocation` (`ActorComponent.GetOwner` (`self.Cube`))))
  (bind _outrownames (`DataTableFunctionLibrary.GetDataTableRowNames` _diseasetableref))
  (for _array_element _outrownames
    (bind _returnvalue (`|GetDataTableRow` _diseasetableref _array_element)
      (:`then`
        (`KismetArrayLibrary.Array_Add` (`self.Cure Type`) _returnvalue)
        (bind _output_get (set `self.Cure` (`.Cure_16_64870F874EE9995440602FB11DECFD0C` (break `/Game/Blueprint/STR_Disease` (`|GetArrayItem` (`self.Cure Type`) (`self.CureNumber`)))))))
      (:`RowNotFound`
        (`KismetSystemLibrary.PrintString` "addObjtable"))))
  (`KismetSystemLibrary.PrintString` "loop done!"))

(event `self.ReceiveActorBeginCursorOver`
  ; over or under
  (`KismetSystemLibrary.PrintString` "over")
  (set `self.MouseOver` true)
  (`KismetSystemLibrary.PrintString` (stale `self.ReceiveBeginPlay` _output_get)))

(event `self.ReceiveActorEndCursorOver`
  ; over or under
  (`KismetSystemLibrary.PrintString` "under")
  (set `self.MouseOver` false))

(event `self.ReceiveTick`
  (params (DeltaSeconds :type "Float (single-precision)"))
  (bind _cube (`self.Cube`))
  (bind _cube_2 (`self.Cube`))
  (bind _worldlocation (`PlayerController.DeprojectMousePositionToWorld` (`GameplayStatics.GetPlayerController` 0)))
  (bind _returnvalue_x (`KismetMathLibrary.BreakVector` (`SceneComponent.K2_GetComponentLocation` _cube)))
  (`|ExecutionSequence`
    (:`then_0`
      ; make him big
      (if (`self.MouseOver`)
        (`SceneComponent.SetRelativeScale3D` _cube_2 (1.0 1.0 1.0))
        (elif (not (`self.bIsDragging`))
          (`SceneComponent.SetRelativeScale3D` _cube_2 (0.5 0.5 0.5)))))
    (:`then_1`
      ; move object with mouse
      (if (`self.bIsDragging`)
        (`SceneComponent.K2_SetWorldLocation` _cube (`KismetMathLibrary.MakeVector` _returnvalue_x (.y _worldlocation) (.z _worldlocation)) false false)))))

(event `self.Cube.OnClicked`
  (params (TouchedComponent :type "PrimitiveComponent Object Reference") (ButtonPressed :type "Key Structure"))
  ; I want that thing
  (set `self.bIsDragging` true))

(event `self.Cube.OnReleased`
  (params (TouchedComponent :type "PrimitiveComponent Object Reference") (ButtonReleased :type "Key Structure"))
  ; object back to origin
  (set `self.bIsDragging` false)
  (`SceneComponent.K2_SetWorldLocation` (`self.Cube`) (`self.Object Origin`) false false))

(fn `UserConstructionScript`)