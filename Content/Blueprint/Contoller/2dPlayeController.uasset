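; A player controller Blueprint, named for a 2D player, that constrains how far the camera can rotate.
; On BeginPlay it stores a cast reference to player controller 0 and sets the camera manager's pitch limits, plus yaw limits symmetric around CurrentFace.
; The limits are set only once, as Tick is empty and nothing here updates CurrentFace.
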(event `self.ReceiveBeginPlay`
  (bind _returnvalue (`GameplayStatics.GetPlayerCameraManager` 0))
  (bind _currentface (`self.CurrentFace`))
  ;[0.05821 0.15 0.0439 0.5] Sets constrains for the camera on BeginPlay
  (set `self.2dPlayerRef` (cast `/Game/Blueprint/Contoller/2dPlayeController` (`GameplayStatics.GetPlayerController` 0) :!pure true))
  (set `PlayerCameraManager.ViewPitchMax` 10.0 _returnvalue)
  (set `PlayerCameraManager.ViewPitchMin` -45.0 _returnvalue)
  (set `PlayerCameraManager.ViewYawMax` (+ _currentface 40.0) _returnvalue)
  (set `PlayerCameraManager.ViewYawMin` (- _currentface 40.0) _returnvalue))

(fn `UserConstructionScript`)